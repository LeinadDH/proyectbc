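; Deck manager Blueprint that handles the player's card deck and hand.
; On BeginPlay it builds the deck from a data table, shuffles it and draws a starting hand.
; PlayCard moves the played card from the hand back into the deck, reshuffles and draws a replacement.
; The UI update is only a debug print placeholder.
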(event `self.ReceiveBeginPlay`
  (bind _builtdeck (`/Game/LazySheeps/DataSets/DeckManager.BuildDeck` (`self.DT_Deck`)))
  (bind _output_get (set `self.Current Deck` _builtdeck))
  (bind _shuffleddeck (`/Game/LazySheeps/DataSets/DeckManager.ShuffleDeck` _output_get))
  (bind _output_get_2 (set `self.Current Deck` _shuffleddeck))
  (for _ (range 3)
    (bind _carddraw (`/Game/LazySheeps/DataSets/DeckManager.DrawCard` _output_get_2))
    (`KismetArrayLibrary.Array_Add` (`self.CardsInHand`) _carddraw)))

(event `PlayCard`
  (params (PlayedCard :type "/Game/LazySheeps/DataSets/S_Base_Card Structure"))
  (`KismetSystemLibrary.PrintString` "PlayedCardevent")
  (`KismetArrayLibrary.Array_RemoveItem` (`self.CardsInHand`) PlayedCard)
  (bind _curretdeck (`/Game/LazySheeps/DataSets/DeckManager.AddCard` PlayedCard (`self.Current Deck`)))
  (bind _shuffleddeck (`/Game/LazySheeps/DataSets/DeckManager.ShuffleDeck` _curretdeck))
  (bind _carddraw (`/Game/LazySheeps/DataSets/DeckManager.DrawCard` _shuffleddeck))
  (`KismetArrayLibrary.Array_Add` (`self.CardsInHand`) _carddraw)
  (`KismetSystemLibrary.PrintString` "UpdateUI"))

(fn `UserConstructionScript`)