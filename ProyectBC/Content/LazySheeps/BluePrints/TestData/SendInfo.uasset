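; SendInfo is a test actor that passes enemy spawn data to the SpawnerController level when it registers a Hit event.
; After a short delay, it writes the enemy count and the array of enemies to spawn into the PersistentData game instance.
; It then adds a fade-out widget and opens the level after another delay, printing debug messages for success or cast failure.
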(event `self.ReceiveHit`
  (params (MyComp :type "PrimitiveComponent Object Reference") (Other :type "Actor Object Reference") (OtherComp :type "PrimitiveComponent Object Reference") (bSelfMoved :type Boolean) (HitLocation :type "Vector Structure") (HitNormal :type "Vector Structure") (NormalImpulse :type "Vector Structure") (Hit :type "HitResult Structure (by ref)"))
  (`KismetSystemLibrary.Delay` 1.0)
  (bind _aspersistent_data (cast `/Game/LazySheeps/BluePrints/GameInstance/PersistentData` (`GameplayStatics.GetGameInstance`))
    (:`then`
      (bind _output_get (set `/Game/LazySheeps/BluePrints/GameInstance/PersistentData.EnemyCuantity` (`self.ArrayLenght`) _aspersistent_data))
      (bind _aspersistent_data_2 (cast `/Game/LazySheeps/BluePrints/GameInstance/PersistentData` (`GameplayStatics.GetGameInstance`))
        (:`then`
          (set `/Game/LazySheeps/BluePrints/GameInstance/PersistentData.EnemiesArray` (`self.EnemiesToSpawn`) _aspersistent_data_2)
          (`KismetSystemLibrary.PrintString` "Correct Send")
          (bind _returnvalue (`|CreateWidget` "/Game/LazySheeps/BluePrints/SceneTransitions/FadeOut.FadeOut_C"))
          (`UserWidget.AddToViewport` _returnvalue 0)
          (`KismetSystemLibrary.Delay` 1.0)
          (`GameplayStatics.OpenLevel` "SpawnerController"))
        (:`CastFailed`
          (`KismetSystemLibrary.PrintString` "Error to send array"))))
    (:`CastFailed`
      (`KismetSystemLibrary.PrintString` "Error to send int"))))

(event `self.ReceiveBeginPlay`)

(fn `UserConstructionScript`)