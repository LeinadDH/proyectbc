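; CharacterController is a pawn Blueprint that lets the player cycle the selected character among UIHPBaseActor instances in the level.
; On BeginPlay it gathers all such actors and selects the one at the current index.
; Q steps forward and E steps back, deselecting the old actor and selecting the new one through SelectCharacter.
; The index wraps over a hardcoded count of four, relying on GetAllActorsOfClass order.
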(event `self.ReceiveTick`
  (params (DeltaSeconds :type "Float (single-precision)")))

(event `self.ReceiveBeginPlay`
  (bind _outactors (`GameplayStatics.GetAllActorsOfClass` "/Game/LazySheeps/BluePrints/Actors/UIHPBaseActor.UIHPBaseActor_C"))
  (bind _output_get (set `self.Out Actors` _outactors))
  (`/Game/LazySheeps/BluePrints/Actors/UIHPBaseActor.SelectCharacter` (`|GetArrayItem` _output_get (`self.SelectedChar`)) true))

(event `Key|Q`
  (params (Key :type "Key Structure"))
  (:`Pressed`
    (`/Game/LazySheeps/BluePrints/Actors/UIHPBaseActor.SelectCharacter` (`|GetArrayItem` (`self.Out Actors`) (`self.SelectedChar`)) false)
    (bind _output_get (set `self.SelectedChar` (+ (`self.SelectedChar`) 1)))
    (if (>= _output_get 4)
      (bind _output_get_2 (set `self.SelectedChar` 0))
      (`/Game/LazySheeps/BluePrints/Actors/UIHPBaseActor.SelectCharacter` (`|GetArrayItem` (`self.Out Actors`) _output_get_2) true)
      (else
        (bind _output_get_3 (set `self.SelectedChar` _output_get))
        (`/Game/LazySheeps/BluePrints/Actors/UIHPBaseActor.SelectCharacter` (`|GetArrayItem` (`self.Out Actors`) _output_get_3) true)))))

(event `Key|E`
  (params (Key :type "Key Structure"))
  (:`Pressed`
    (`/Game/LazySheeps/BluePrints/Actors/UIHPBaseActor.SelectCharacter` (`|GetArrayItem` (`self.Out Actors`) (`self.SelectedChar`)) false)
    (bind _output_get (set `self.SelectedChar` (- (`self.SelectedChar`) 1)))
    (if (< _output_get 0)
      (bind _output_get_2 (set `self.SelectedChar` 3))
      (`/Game/LazySheeps/BluePrints/Actors/UIHPBaseActor.SelectCharacter` (`|GetArrayItem` (`self.Out Actors`) _output_get_2) true)
      (else
        (bind _output_get_3 (set `self.SelectedChar` _output_get))
        (`/Game/LazySheeps/BluePrints/Actors/UIHPBaseActor.SelectCharacter` (`|GetArrayItem` (`self.Out Actors`) _output_get_3) true)))))

(fn `UserConstructionScript`)