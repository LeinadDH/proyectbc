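; HPTestPawn is a test pawn that changes health values for four actors from the keyboard.
; Each actor has a key pair (Q/E, A/D, Z/C, 1/3) that lowers or raises its own health variable by a fixed step.
; Results are clamped between zero and MaxHealt, except actor two's decrease, which uses its current health as the upper bound.
; The pawn only stores these values, with no other active logic.
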(event `Key|Z`
  (params (Key :type "Key Structure"))
  ;[1 1 1] Input Actor Three
  (:`Pressed`
    (set `self.CurrentHealtA3` (`KismetMathLibrary.FClamp` (- (`self.CurrentHealtA3`) 100.0) 0.0 (`self.MaxHealt`)))))

(event `Key|Q`
  (params (Key :type "Key Structure"))
  ;[1 1 1] Input Actor One
  (:`Pressed`
    (set `self.CurrentHealtA1` (`KismetMathLibrary.FClamp` (- (`self.CurrentHealtA1`) 100.0) 0.0 (`self.MaxHealt`)))))

(event `Key|C`
  (params (Key :type "Key Structure"))
  ;[1 1 1] Input Actor Three
  (:`Pressed`
    (set `self.CurrentHealtA3` (`KismetMathLibrary.FClamp` (+ (`self.CurrentHealtA3`) 100.0) 0.0 (`self.MaxHealt`)))))

(event `Key|E`
  (params (Key :type "Key Structure"))
  ;[1 1 1] Input Actor One
  (:`Pressed`
    (set `self.CurrentHealtA1` (`KismetMathLibrary.FClamp` (+ (`self.CurrentHealtA1`) 100.0) 0.0 (`self.MaxHealt`)))))

(event `Key|One`
  (params (Key :type "Key Structure"))
  ;[1 1 1] Input Actor Four
  (:`Pressed`
    (set `self.CurrentHealtA4` (`KismetMathLibrary.FClamp` (- (`self.CurrentHealtA4`) 100.0) 0.0 (`self.MaxHealt`)))))

(event `Key|A`
  (params (Key :type "Key Structure"))
  ;[1 1 1] Input Actor Two
  (:`Pressed`
    (set `self.CurrentHealtA2` (`KismetMathLibrary.FClamp` (- (`self.CurrentHealtA2`) 100.0) 0.0 (`self.CurrentHealtA2`)))))

(event `Key|Three`
  (params (Key :type "Key Structure"))
  ;[1 1 1] Input Actor Four
  (:`Pressed`
    (set `self.CurrentHealtA4` (`KismetMathLibrary.FClamp` (+ (`self.CurrentHealtA4`) 100.0) 0.0 (`self.MaxHealt`)))))

(event `Key|D`
  (params (Key :type "Key Structure"))
  ;[1 1 1] Input Actor Two
  (:`Pressed`
    (set `self.CurrentHealtA2` (`KismetMathLibrary.FClamp` (+ (`self.CurrentHealtA2`) 100.0) 0.0 (`self.MaxHealt`)))))

(fn `UserConstructionScript`)