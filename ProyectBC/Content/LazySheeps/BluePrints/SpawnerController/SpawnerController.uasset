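; SpawnerController is a Blueprint that holds the spawn locations for enemies and players.
; On BeginPlay it caches the world transforms of three enemy and three player spawn points into two arrays.
; The spawning logic is unfinished: a loop over enemy points, a SpawnActor node and a count comparison are left unconnected, so nothing spawns here.
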(event `self.ReceiveBeginPlay`
  (`|ExecutionSequence`
    (:`then_0`
      (bind _output_get (set `self.enemiesSpawnPoints` (`|MakeArray` (`SceneComponent.K2_GetComponentToWorld` (`self.SpawnPoint_Enemy_1`)) (`SceneComponent.K2_GetComponentToWorld` (`self.SpawnPoint_Enemy_2`)) (`SceneComponent.K2_GetComponentToWorld` (`self.SpawnPoint_Enemy_3`)))))
      (if true
        _))
    (:`then_1`
      (set `self.playersSpawnPoints` (`|MakeArray` (`SceneComponent.K2_GetComponentToWorld` (`self.SpawnPoint_Player_1`)) (`SceneComponent.K2_GetComponentToWorld` (`self.SpawnPoint_Player_2`)) (`SceneComponent.K2_GetComponentToWorld` (`self.SpawnPoint_Player_3`)))))))

(fn `UserConstructionScript`)